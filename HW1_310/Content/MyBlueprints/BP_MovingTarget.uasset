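; Shooting target that slides back and forth along X and shows its health on a widget component.
; A timeline lerps it between offsets either side of its spawn point, reversing through a FlipFlop and re-caching the widget every update.
; Projectile hits subtract fixed health and update the bar; at zero it increments the player's TargetsHit, calls CheckGoal and destroys itself.
; AnyDamage only lowers health, and UpdateHealthBar is not called here.
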(event `self.ReceiveHit`
  (params (MyComp :type "PrimitiveComponent Object Reference") (Other :type "Actor Object Reference") (OtherComp :type "PrimitiveComponent Object Reference") (bSelfMoved :type Boolean) (HitLocation :type "Vector Structure") (HitNormal :type "Vector Structure") (NormalImpulse :type "Vector Structure") (Hit :type "HitResult Structure (by ref)"))
  (cast `/Game/FirstPerson/Blueprints/BP_FirstPersonProjectile` Other)
  (bind _asbp_first_person_character (cast `/Game/FirstPerson/Blueprints/BP_FirstPersonCharacter` (`GameplayStatics.GetPlayerCharacter` 0)))
  (bind _output_get (set `self.CurrentHealth` (`KismetMathLibrary.FClamp` (- (`self.CurrentHealth`) 20.0) 0.0 (`self.MaxHealth`))))
  (`ProgressBar.SetPercent` (`/Game/UI/TargetHealthWidget.Target_Health_Bar` (stale `self.ReceiveBeginPlay` _output_get_3)) (`KismetMathLibrary.SafeDivide` _output_get (`self.MaxHealth`)))
  (`/Engine/EditorBlueprintResources/StandardMacros.CompareFloat` (`self.CurrentHealth`)
    (:`==`
      _)
    (:`<`
      _))
  (`/Engine/EditorBlueprintResources/StandardMacros.IncrementInt` (`/Game/FirstPerson/Blueprints/BP_FirstPersonCharacter.TargetsHit` _asbp_first_person_character)
    (:`  `
      (`/Game/FirstPerson/Blueprints/BP_FirstPersonCharacter.CheckGoal` _asbp_first_person_character)
      (`self.K2_DestroyActor`))))

(event `self.ReceiveBeginPlay`
  (bind _returnvalue (`self.K2_GetActorLocation`))
  (bind _output_get (set `self.StartLocation` (+ _returnvalue (100.0 -0.0 0.0))))
  (bind _output_get_2 (set `self.EndLocation` (+ _returnvalue (-100.0 0.0 0.0))))
  (bind (_direction _newtrack_0) (`Timeline|Timeline` :!via `PlayFromStart` :!label _label)
    (:`Update`
      (`self.K2_SetActorLocation` (`KismetMathLibrary.VLerp` _output_get _output_get_2 _newtrack_0))
      (bind _astarget_health_widget (cast `/Game/UI/TargetHealthWidget` (`WidgetComponent.GetUserWidgetObject` (`self.HealthWidget`))))
      (bind _output_get_3 (set `self.As Target Health Widget` _astarget_health_widget)))
    (:`Finished`
      (`/Engine/EditorBlueprintResources/StandardMacros.FlipFlop`
        (:`A`
          (goto _label :!via `Reverse`))
        (:`B`
          (goto _label))))))

(event `self.ReceiveAnyDamage`
  (params (Damage :type "Float (single-precision)") (DamageType :type "DamageType Object Reference") (InstigatedBy :type "Controller Object Reference") (DamageCauser :type "Actor Object Reference"))
  (set `self.CurrentHealth` (- (`self.CurrentHealth`) Damage)))

(fn `UpdateHealthBar`
  (bind _astarget_health_widget (cast `/Game/UI/TargetHealthWidget` (`WidgetComponent.GetUserWidgetObject` (`self.HealthWidget`))))
  (`ProgressBar.SetPercent` (`/Game/UI/TargetHealthWidget.Target_Health_Bar` _astarget_health_widget) (/ (`self.CurrentHealth`) (`self.MaxHealth`))))

(fn `UserConstructionScript`)